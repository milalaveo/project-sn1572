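; BP_Intel is a collectible intel pickup that the player gathers by interacting with it.
; Its sphere collision adds it to the overlapping BP_FirstPersonCharacter's InteractableObject collection on entry and removes it on exit.
; When UseInteractableObject fires, it calls GatherIntel on GM_MyFirstSuperGame and destroys itself.
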(event `self.ShpereCollision.OnComponentBeginOverlap`
  (params (OverlappedComponent :type "PrimitiveComponent Object Reference") (OtherActor :type "Actor Object Reference") (OtherComp :type "PrimitiveComponent Object Reference") (OtherBodyIndex :type Integer) (bFromSweep :type Boolean) (SweepResult :type "HitResult Structure (by ref)"))
  (bind _asbp_first_person_character (cast `/Game/FirstPerson/Blueprints/BP_FirstPersonCharacter` OtherActor))
  (`KismetArrayLibrary.Array_Add` (`/Game/FirstPerson/Blueprints/BP_FirstPersonCharacter.InteractableObject` _asbp_first_person_character) self))

(event `self.ShpereCollision.OnComponentEndOverlap`
  (params (OverlappedComponent :type "PrimitiveComponent Object Reference") (OtherActor :type "Actor Object Reference") (OtherComp :type "PrimitiveComponent Object Reference") (OtherBodyIndex :type Integer))
  (bind _asbp_first_person_character (cast `/Game/FirstPerson/Blueprints/BP_FirstPersonCharacter` OtherActor))
  (`KismetArrayLibrary.Array_RemoveItem` (`/Game/FirstPerson/Blueprints/BP_FirstPersonCharacter.InteractableObject` _asbp_first_person_character) self))

(event `/Game/MyFirstSuperGame/Intel/BPI_Interaction.UseInteractableObject`
  (bind _asgm_my_first_super_game (cast `/Game/MyFirstSuperGame/Framework/GM_MyFirstSuperGame` (`GameplayStatics.GetGameMode`)))
  (`/Game/MyFirstSuperGame/Framework/GM_MyFirstSuperGame.Gather Intel` _asgm_my_first_super_game)
  (`self.K2_DestroyActor`))

(fn `UserConstructionScript`)