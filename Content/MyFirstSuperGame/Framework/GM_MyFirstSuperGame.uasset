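; Game mode that runs the match flow for an intel-gathering game with guard enemies.
; HandleNewSuperGameState is a change-guarded state machine, stepping automatically from setup through a pass-through standby and start into an empty in-progress state.
; Setup counts BP_Intel actors, start switches every Enemy's guard state, and end prints the result, with a sound on a win.
; Gather and completion-check functions track intel; nothing here triggers the end state.
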(event `self.ReceiveBeginPlay`
  (`self.HandleNewSuperGameState` "NewEnumerator1"))

(event `SetupPhase`
  (bind _outactors (`GameplayStatics.GetAllActorsOfClass` "/Game/MyFirstSuperGame/Intel/BP_Intel.BP_Intel_C"))
  (set `self.TotalIntel` (`KismetArrayLibrary.Array_Length` _outactors))
  (`KismetSystemLibrary.Delay` 1.0)
  (`self.HandleNewSuperGameState` "NewEnumerator2"))

(event `StandByPhase`
  (`self.HandleNewSuperGameState` "NewEnumerator3"))

(event `StartTheGame`
  (`|ExecutionSequence`
    (:`then_0`
      (bind _outactors (`GameplayStatics.GetAllActorsOfClass` "/Game/MyFirstSuperGame/Enemy/Enemy.Enemy_C"))
      (for _array_element _outactors
        (`/Game/MyFirstSuperGame/Enemy/Enemy.HandleNewGuardState` _array_element "NewEnumerator2")))
    (:`then_1`
      (`self.HandleNewSuperGameState` "NewEnumerator4"))))

(event `GameIsInProgress`)

(event `EndGame`
  (params (WinLoseState :type "/Game/MyFirstSuperGame/Framework/E_WinLoseState Enum" :default "NewEnumerator0"))
  (`KismetSystemLibrary.PrintString` "Game Over!" true true (struct :`R` 0.362458 :`G` 1.0 :`A` 1.0))
  (switch `/Game/MyFirstSuperGame/Framework/E_WinLoseState` WinLoseState
    (:`NewEnumerator1`
      (`KismetSystemLibrary.PrintString` "Pobeda!")
      (`GameplayStatics.PlaySoundAtLocation` "/Game/MyFirstSuperGame/Sounds/standing-here-i-realize_B7hEFlm.standing-here-i-realize_B7hEFlm" (`self.K2_GetActorLocation` (`GameplayStatics.GetPlayerCharacter` 0)) (struct) 1.0 1.0 0.0 null null null null))
    (:`NewEnumerator2`
      (`KismetSystemLibrary.PrintString` "Loh"))))

(fn `CheckIfAllTheIntelIsGathered`
  (returns (ReturnValue :type Boolean))
  (return (>= (`self.IntelGathered`) (`self.TotalIntel`))))

(fn `Gather Intel`
  (set `self.IntelGathered` (+ (`self.IntelGathered`) 1))
  (`KismetSystemLibrary.PrintString` "Got one"))

(fn `HandleNewSuperGameState`
  (params (NewShooterGameState :type "/Game/MyFirstSuperGame/Framework/E_ShooterGameState Enum" :default "NewEnumerator0") (WinLoseState :type "/Game/MyFirstSuperGame/Framework/E_WinLoseState Enum" :default "NewEnumerator0"))
  (if (`|EnumInequality` NewShooterGameState (`self.ShooterGameState`))
    (bind _output_get (set `self.ShooterGameState` NewShooterGameState))
    (switch `/Game/MyFirstSuperGame/Framework/E_ShooterGameState` _output_get
      (:`NewEnumerator1`
        (`self.SetupPhase`))
      (:`NewEnumerator2`
        (`self.StandByPhase`))
      (:`NewEnumerator3`
        (`self.StartTheGame`))
      (:`NewEnumerator4`
        (`self.GameIsInProgress`))
      (:`NewEnumerator5`
        (`self.EndGame` WinLoseState)))))

(fn `UserConstructionScript`)